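; CROC_ADULT_BP is the adult-stage crocodile pet character, built on a parent class that it extends with croc-specific sprites and identity.
; SettingFlipbook assigns the idle, walk left, walk right and attack flipbooks to inherited variables and starts the main sprite on idle.
; On BeginPlay it runs the parent logic, applies those flipbooks, then writes its state and "CROC" pet line to the GAME_INSTANCE.
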(event `self.ReceiveActorBeginOverlap`
  (params (OtherActor :type "Actor Object Reference"))
  (`parent.ReceiveActorBeginOverlap` OtherActor))

(event `self.ReceiveBeginPlay`
  ;[1 1 1] begin play
  (`parent.ReceiveBeginPlay`)
  (`self.setting flipbook`)
  (bind _asgame_instance (cast `/Game/D-PET/GAME_INSTANCE` (`GameplayStatics.GetGameInstance`)))
  (set `/Game/D-PET/GAME_INSTANCE.state` (`self.STATE`) _asgame_instance)
  (bind _output_get (set `self.PET LINE` "CROC"))
  (set `/Game/D-PET/GAME_INSTANCE.pet line` _output_get _asgame_instance))

(event `setting flipbook`
  ;[1 1 1] setting sprite and stage
  (set `self.IDLE FLIPBOOK` "/Game/D-PET/CHARACTERS/CROC/CROC_2_ADULT/IDLE/CROC_ADULT_IDLE_FLIPBOOK.CROC_ADULT_IDLE_FLIPBOOK")
  (set `self.WALK RIGHT FLIPBOOK` "/Game/D-PET/CHARACTERS/CROC/CROC_2_ADULT/WALK/RIGHT/CROC_ADULT_WALK_RIGHT_FLIPBOOK.CROC_ADULT_WALK_RIGHT_FLIPBOOK")
  (set `self.WALK LEFT FLIPBOOK` "/Game/D-PET/CHARACTERS/CROC/CROC_2_ADULT/WALK/LEFT/CROC_ADULT_WALK_LEFT_FLIPBOOK.CROC_ADULT_WALK_LEFT_FLIPBOOK")
  (set `self.ATTACK FLIPBOOK` "/Game/D-PET/CHARACTERS/CROC/CROC_2_ADULT/ATTACK/CROC_ADULT_ATTACK_FLIPBOOK.CROC_ADULT_ATTACK_FLIPBOOK")
  (`PaperFlipbookComponent.SetFlipbook` (`self.MAIN SPRITE`) (`self.IDLE FLIPBOOK`)))

(fn `UserConstructionScript`
  (`parent.UserConstructionScript`))