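; Crocodile character Blueprint for D-PET that gives the creature its Paper2D look for each of its three growth stages.
; On BeginPlay it runs the parent logic, then SetSprite uses the inherited or member STATE value to pick idle, walk-left, walk-right and attack flipbooks.
; The chosen idle flipbook is applied to MAINSPRITE.
; Tick only forwards to the parent class.
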(event `self.ReceiveTick`
  (params (DeltaSeconds :type "Float (single-precision)"))
  (`parent.ReceiveTick` DeltaSeconds))

(event `self.ReceiveBeginPlay`
  ;[1 1 1] begin play
  (`parent.ReceiveBeginPlay`)
  (`self.set sprite`))

(event `set sprite`
  ;[1 1 1] setting sprite and stage
  (if (== (`self.STATE`) 1.0)
    (set `self.IDLE FLIPBOOK` "/Game/D-PET/CHARACTERS/CROC/CROC_1_CHILD/IDLE/CROC_CHILD_IDLE_FLIPBOOK.CROC_CHILD_IDLE_FLIPBOOK")
    (set `self.WALK RIGHT FLIPBOOK` "/Game/D-PET/CHARACTERS/CROC/CROC_1_CHILD/WALK/RIGHT/CROC_CHILD_RUN_RIGHT_FLIPBOOK.CROC_CHILD_RUN_RIGHT_FLIPBOOK")
    (set `self.WALK LEFT FLIPBOOK` "/Game/D-PET/CHARACTERS/CROC/CROC_1_CHILD/WALK/LEFT/CROC_CHILD_RUN_LEFT_FLIPBOOK.CROC_CHILD_RUN_LEFT_FLIPBOOK")
    (set `self.ATTACK FLIPBOOK` "/Game/D-PET/CHARACTERS/CROC/CROC_1_CHILD/ATTACK/CROC_CHILD_ATTACK_FLIPBOOK.CROC_CHILD_ATTACK_FLIPBOOK")
    (`PaperFlipbookComponent.SetFlipbook` (`self.MAIN SPRITE`) (`self.IDLE FLIPBOOK`) :!label _label)
    (elif (== (`self.STATE`) 2.0)
      (set `self.IDLE FLIPBOOK` "/Game/D-PET/CHARACTERS/CROC/CROC_2_ADULT/IDLE/CROC_ADULT_IDLE_FLIPBOOK.CROC_ADULT_IDLE_FLIPBOOK")
      (set `self.WALK RIGHT FLIPBOOK` "/Game/D-PET/CHARACTERS/CROC/CROC_2_ADULT/WALK/RIGHT/CROC_ADULT_WALK_RIGHT_FLIPBOOK.CROC_ADULT_WALK_RIGHT_FLIPBOOK")
      (set `self.WALK LEFT FLIPBOOK` "/Game/D-PET/CHARACTERS/CROC/CROC_2_ADULT/WALK/LEFT/CROC_ADULT_WALK_LEFT_FLIPBOOK.CROC_ADULT_WALK_LEFT_FLIPBOOK")
      (set `self.ATTACK FLIPBOOK` "/Game/D-PET/CHARACTERS/CROC/CROC_2_ADULT/ATTACK/CROC_ADULT_ATTACK_FLIPBOOK.CROC_ADULT_ATTACK_FLIPBOOK")
      (goto _label)
      (elif (== (`self.STATE`) 3.0)
        (set `self.IDLE FLIPBOOK` "/Game/D-PET/CHARACTERS/CROC/CROC_3_MEGA/IDLE/CROC_IDLE_FLIPBOOK.CROC_IDLE_FLIPBOOK")
        (set `self.WALK RIGHT FLIPBOOK` "/Game/D-PET/CHARACTERS/CROC/CROC_3_MEGA/WALK/RIGHT/CROC_RIGHT_FLIPBOOK.CROC_RIGHT_FLIPBOOK")
        (set `self.WALK LEFT FLIPBOOK` "/Game/D-PET/CHARACTERS/CROC/CROC_3_MEGA/WALK/LEFT/CROC_LEFT_FLIPBOOK.CROC_LEFT_FLIPBOOK")
        (set `self.ATTACK FLIPBOOK` "/Game/D-PET/CHARACTERS/CROC/CROC_3_MEGA/ATTACK/CROC_ATTACK_FLIPBOOK.CROC_ATTACK_FLIPBOOK")
        (goto _label)))))

(fn `UserConstructionScript`
  (`parent.UserConstructionScript`))