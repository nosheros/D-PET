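; CROC_MEGA_BP is a croc pet Blueprint, apparently the Mega stage of its line, built on a parent class's sprite and state variables.
; On BeginPlay it assigns the croc idle, walk left/right and attack flipbooks and shows idle on MAINSPRITE.
; It then writes its STATE and a pet line of 1 to the GAME_INSTANCE.
; Tick and overlap events only defer to the parent.
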(event `self.ReceiveActorBeginOverlap`
  (params (OtherActor :type "Actor Object Reference"))
  (`parent.ReceiveActorBeginOverlap` OtherActor))

(event `self.ReceiveBeginPlay`
  ;[1 1 1] begin play
  (`parent.ReceiveBeginPlay`)
  (`self.setting flipbook`)
  (bind _asgame_instance (cast `/Game/D-PET/GAME_INSTANCE` (`GameplayStatics.GetGameInstance`)))
  (set `/Game/D-PET/GAME_INSTANCE.state` (`self.STATE`) _asgame_instance)
  (bind _output_get (set `self.PET LINE` 1.0))
  (set `/Game/D-PET/GAME_INSTANCE.pet line` _output_get _asgame_instance))

(event `setting flipbook`
  ;[1 1 1] setting sprite and stage
  (set `self.IDLE FLIPBOOK` "/Game/D-PET/CHARACTERS/CROC/CROC_3_MEGA/IDLE/CROC_IDLE_FLIPBOOK.CROC_IDLE_FLIPBOOK")
  (set `self.WALK RIGHT FLIPBOOK` "/Game/D-PET/CHARACTERS/CROC/CROC_3_MEGA/WALK/RIGHT/CROC_RIGHT_FLIPBOOK.CROC_RIGHT_FLIPBOOK")
  (set `self.WALK LEFT FLIPBOOK` "/Game/D-PET/CHARACTERS/CROC/CROC_3_MEGA/WALK/LEFT/CROC_LEFT_FLIPBOOK.CROC_LEFT_FLIPBOOK")
  (set `self.ATTACK FLIPBOOK` "/Game/D-PET/CHARACTERS/CROC/CROC_3_MEGA/ATTACK/CROC_ATTACK_FLIPBOOK.CROC_ATTACK_FLIPBOOK")
  (`PaperFlipbookComponent.SetFlipbook` (`self.MAIN SPRITE`) (`self.IDLE FLIPBOOK`)))

(fn `UserConstructionScript`
  (`parent.UserConstructionScript`))