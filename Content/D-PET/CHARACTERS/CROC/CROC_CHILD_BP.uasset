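; Child-stage crocodile pet character for the D-PET game, a Blueprint child that inherits its behaviour from a parent pet class.
; On BeginPlay it runs the parent logic, assigns the croc child idle, run and attack flipbooks, and sets the sprite to idle.
; It then writes its state and a pet line of 1 to the game instance.
; The movement event is left empty and the parent overlap call is disabled.
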(event `self.ReceiveTick`
  (params (DeltaSeconds :type "Float (single-precision)"))
  (`parent.ReceiveTick` DeltaSeconds))

(event `movement function`)

(event `self.ReceiveBeginPlay`
  ;[1 1 1] begin play
  (`parent.ReceiveBeginPlay`)
  (`self.setting flipbook`)
  (bind _asgame_instance (cast `/Game/D-PET/GAME_INSTANCE` (`GameplayStatics.GetGameInstance`)))
  (set `/Game/D-PET/GAME_INSTANCE.state` (`self.STATE`) _asgame_instance)
  (bind _output_get (set `self.PET LINE` 1.0))
  (set `/Game/D-PET/GAME_INSTANCE.pet line` _output_get _asgame_instance))

(event `setting flipbook`
  ;[1 1 1] setting sprite and stage
  (set `self.IDLE FLIPBOOK` "/Game/D-PET/CHARACTERS/CROC/CROC_1_CHILD/IDLE/CROC_CHILD_IDLE_FLIPBOOK.CROC_CHILD_IDLE_FLIPBOOK")
  (set `self.WALK RIGHT FLIPBOOK` "/Game/D-PET/CHARACTERS/CROC/CROC_1_CHILD/WALK/RIGHT/CROC_CHILD_RUN_RIGHT_FLIPBOOK.CROC_CHILD_RUN_RIGHT_FLIPBOOK")
  (set `self.WALK LEFT FLIPBOOK` "/Game/D-PET/CHARACTERS/CROC/CROC_1_CHILD/WALK/LEFT/CROC_CHILD_RUN_LEFT_FLIPBOOK.CROC_CHILD_RUN_LEFT_FLIPBOOK")
  (set `self.ATTACK FLIPBOOK` "/Game/D-PET/CHARACTERS/CROC/CROC_1_CHILD/ATTACK/CROC_CHILD_ATTACK_FLIPBOOK.CROC_CHILD_ATTACK_FLIPBOOK")
  (`PaperFlipbookComponent.SetFlipbook` (`self.MAIN SPRITE`) (`self.IDLE FLIPBOOK`)))

(fn `UserConstructionScript`
  (`parent.UserConstructionScript`))