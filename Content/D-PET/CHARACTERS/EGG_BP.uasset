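; EGG_BP is an egg actor for the D-PET game that ages toward hatching and spawns a child creature.
; AGING decrements AGE on a re-armed one-second timer, then shows the HATCH_BUTTON widget at zero.
; HATCH removes that widget, randomly picks a line from LINECHOOSER, spawns the child and destroys the egg.
; All four line branches currently spawn CROC_CHILD_BP at the egg's transform.
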(event `self.ReceiveBeginPlay`
  (`self.AGING`))

(event `AGING`
  (bind _output_get (set `self.AGE` (- (`self.AGE`) 1.0)))
  (if (<= _output_get 0.0)
    (bind _returnvalue (`|CreateWidget` "/Game/D-PET/WIDGET/HATCH_BUTTON.HATCH_BUTTON_C"))
    (`UserWidget.AddToViewport` _returnvalue 0)
    (else
      (`KismetSystemLibrary.K2_SetTimerDelegate` (delegate `AGING`) 1.0))))

(event `HATCH`
  (bind _foundwidgets (`WidgetBlueprintLibrary.GetAllWidgetsOfClass` "/Game/D-PET/WIDGET/HATCH_BUTTON.HATCH_BUTTON_C" false))
  (`Widget.RemoveFromParent` _foundwidgets)
  (bind _output_get (set `self.CHOSEN LINE` (`|GetArrayItem` (`self.LINE CHOOSER`) (`KismetMathLibrary.RandomInteger` 4))))
  (if (== _output_get 0)
    (`|SpawnActorFromClass` "/Game/D-PET/CHARACTERS/CROC/CROC_CHILD_BP.CROC_CHILD_BP_C" (`SceneComponent.K2_GetComponentToWorld` (`self.DefaultSceneRoot`)) "Undefined" "MultiplyWithRoot" null null)
    (`self.K2_DestroyActor` :!label _label)
    (elif (== _output_get 1)
      (`|SpawnActorFromClass` "/Game/D-PET/CHARACTERS/CROC/CROC_CHILD_BP.CROC_CHILD_BP_C" (`SceneComponent.K2_GetComponentToWorld` (`self.DefaultSceneRoot`)) "Undefined" "MultiplyWithRoot" null null)
      (goto _label)
      (elif (== _output_get 2)
        (`|SpawnActorFromClass` "/Game/D-PET/CHARACTERS/CROC/CROC_CHILD_BP.CROC_CHILD_BP_C" (`SceneComponent.K2_GetComponentToWorld` (`self.DefaultSceneRoot`)) "Undefined" "MultiplyWithRoot" null null)
        (goto _label)
        (elif (== _output_get 3)
          (`|SpawnActorFromClass` "/Game/D-PET/CHARACTERS/CROC/CROC_CHILD_BP.CROC_CHILD_BP_C" (`SceneComponent.K2_GetComponentToWorld` (`self.DefaultSceneRoot`)) "Undefined" "MultiplyWithRoot" null null)
          (goto _label))))))

(fn `UserConstructionScript`)