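; Base character Blueprint for a virtual pet that wanders, ages and evolves, using a flipbook sprite.
; Timers alternate random AI moves with idle pauses and increment age; at the threshold, state rises and an evolution button appears.
; EVOLVEPET checks fight count, then replaces the actor by state, though every pet line currently spawns Croc classes.
; Hovering halts walking, clicking opens a widget, and BeginPlay saves pet stats to a slot.
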(event `self.ReceiveTick`
  (params (DeltaSeconds :type "Float (single-precision)")))

(event `movement`
  ;[1 1 1] movement
  (if (== (`KismetMathLibrary.RandomInteger` (`self.INTEGER FOR MOVEMENT`)) 0)
    (`PaperFlipbookComponent.SetFlipbook` (`self.MAIN SPRITE`) (`self.WALK RIGHT FLIPBOOK`))
    (else
      (`PaperFlipbookComponent.SetFlipbook` (`self.MAIN SPRITE`) (`self.WALK LEFT FLIPBOOK`))))
  (`|AIMoveTo` self (`NavigationSystemV1.K2_GetRandomReachablePointInRadius` (`self.K2_GetActorLocation`) 5000.0 null null) null
    (:`OnSuccess`
      (`KismetSystemLibrary.K2_SetTimerDelegate` (delegate `wait movement`) 5.0))))

(event `wait movement`
  ;[1 1 1] movement
  (`PaperFlipbookComponent.SetFlipbook` (`self.MAIN SPRITE`) (`self.IDLE FLIPBOOK`))
  (`KismetSystemLibrary.K2_SetTimerDelegate` (delegate `movement`) 5.0))

(event `self.ReceiveBeginPlay`
  ;[1 1 1] begin play
  (`self.AGING`)
  (`self.movement`)
  (`self.SAVE DATA`)
  (`WidgetBlueprintLibrary.SetInputMode_GameAndUIEx` null null)
  (set `PlayerController.bEnableMouseOverEvents` true (`GameplayStatics.GetPlayerController` 0)))

(event `self.MAIN SPRITE.OnBeginCursorOver`
  (params (TouchedComponent :type "PrimitiveComponent Object Reference"))
  (set `CharacterMovementComponent.MaxWalkSpeed` 0.0 (`self.CharacterMovement`))
  (`KismetSystemLibrary.PrintString` "Hello"))

(event `self.MAIN SPRITE.OnEndCursorOver`
  (params (TouchedComponent :type "PrimitiveComponent Object Reference"))
  (set `CharacterMovementComponent.MaxWalkSpeed` 600.0 (`self.CharacterMovement`))
  (`KismetSystemLibrary.PrintString` "goodbye"))

(event `self.MAIN SPRITE.OnClicked`
  (params (TouchedComponent :type "PrimitiveComponent Object Reference") (ButtonPressed :type "Key Structure"))
  (bind _returnvalue (`|CreateWidget` "/Game/D-PET/WIDGET/STATS_SCREEN.STATS_SCREEN_C"))
  (`UserWidget.AddToViewport` _returnvalue 0))

(event `AGING`
  ;[1 1 1] aging
  (bind _output_get (set `self.AGE` (+ (`self.AGE`) 1.0)))
  (if (>= _output_get 10.0)
    (set `self.STATE` (+ (`self.STATE`) 1.0))
    (bind _asd_pet_game_instance (cast `/Game/D-PET/D_PET_GAME_INSTANCE` (`GameplayStatics.GetGameInstance`)))
    (set `/Game/D-PET/D_PET_GAME_INSTANCE.state` (`self.STATE`) _asd_pet_game_instance)
    (bind _returnvalue (`|CreateWidget` "/Game/D-PET/WIDGET/EVOLUTION_BUTTON.EVOLUTION_BUTTON_C"))
    (`UserWidget.AddToViewport` _returnvalue 0)
    (else
      (bind _asd_pet_game_instance_2 (cast `/Game/D-PET/D_PET_GAME_INSTANCE` (`GameplayStatics.GetGameInstance`)))
      (set `/Game/D-PET/D_PET_GAME_INSTANCE.AGE` (`self.AGE`) _asd_pet_game_instance_2)
      (`KismetSystemLibrary.K2_SetTimerDelegate` (delegate `AGING`) 60.0))))

(event `EVOLVE PET`
  (if (>= (`self.FIGHTS`) 10.0)
    (`self.CHECK LINE AND STATE`)))

(fn `CHECK LINE AND STATE`
  (bind _state (`self.STATE`))
  (bind _state_2 (`self.STATE`))
  (bind _state_3 (`self.STATE`))
  (bind _pet_line (`self.PET LINE`))
  (if (== _pet_line "CROC")
    (if (<= _state_2 1.0)
      (`self.K2_DestroyActor`)
      (`|SpawnActorFromClass` "/Game/D-PET/CHARACTERS/CROC/CROC_CHILD_BP.CROC_CHILD_BP_C" (`SceneComponent.K2_GetComponentToWorld` (`self.CapsuleComponent`)) "Undefined" "MultiplyWithRoot" null null)
      (elif (== _state_2 2.0)
        (`self.K2_DestroyActor`)
        (`|SpawnActorFromClass` "/Game/D-PET/CHARACTERS/CROC/CROC_ADULT_BP.CROC_ADULT_BP_C" (`SceneComponent.K2_GetComponentToWorld` (`self.CapsuleComponent`)) "Undefined" "MultiplyWithRoot" null null)
        (elif (>= _state_2 3.0)
          (`self.K2_DestroyActor`)
          (`|SpawnActorFromClass` "/Game/D-PET/CHARACTERS/CROC/CROC_MEGA_BP.CROC_MEGA_BP_C" (`SceneComponent.K2_GetComponentToWorld` (`self.CapsuleComponent`)) "Undefined" "MultiplyWithRoot" null null))))
    (elif (== _pet_line "SNAKE")
      (if (<= _state_3 1.0)
        (`self.K2_DestroyActor`)
        (`|SpawnActorFromClass` "/Game/D-PET/CHARACTERS/CROC/CROC_CHILD_BP.CROC_CHILD_BP_C" (`SceneComponent.K2_GetComponentToWorld` (`self.CapsuleComponent`)) "Undefined" "MultiplyWithRoot" null null)
        (elif (== _state_3 2.0)
          (`self.K2_DestroyActor`)
          (`|SpawnActorFromClass` "/Game/D-PET/CHARACTERS/CROC/CROC_ADULT_BP.CROC_ADULT_BP_C" (`SceneComponent.K2_GetComponentToWorld` (`self.CapsuleComponent`)) "Undefined" "MultiplyWithRoot" null null)
          (elif (>= _state_3 3.0)
            (`self.K2_DestroyActor`)
            (`|SpawnActorFromClass` "/Game/D-PET/CHARACTERS/CROC/CROC_MEGA_BP.CROC_MEGA_BP_C" (`SceneComponent.K2_GetComponentToWorld` (`self.CapsuleComponent`)) "Undefined" "MultiplyWithRoot" null null))))
      (elif (== _pet_line "OGRE")
        (if (<= _state 1.0)
          (`self.K2_DestroyActor`)
          (`|SpawnActorFromClass` "/Game/D-PET/CHARACTERS/CROC/CROC_CHILD_BP.CROC_CHILD_BP_C" (`SceneComponent.K2_GetComponentToWorld` (`self.CapsuleComponent`)) "Undefined" "MultiplyWithRoot" null null)
          (elif (== _state 2.0)
            (`self.K2_DestroyActor`)
            (`|SpawnActorFromClass` "/Game/D-PET/CHARACTERS/CROC/CROC_ADULT_BP.CROC_ADULT_BP_C" (`SceneComponent.K2_GetComponentToWorld` (`self.CapsuleComponent`)) "Undefined" "MultiplyWithRoot" null null)
            (elif (>= _state 3.0)
              (`self.K2_DestroyActor`)
              (`|SpawnActorFromClass` "/Game/D-PET/CHARACTERS/CROC/CROC_MEGA_BP.CROC_MEGA_BP_C" (`SceneComponent.K2_GetComponentToWorld` (`self.CapsuleComponent`)) "Undefined" "MultiplyWithRoot" null null))))))))

(fn `SAVE DATA`
  (bind _returnvalue (`GameplayStatics.CreateSaveGameObject` "/Game/D-PET/CHARACTERS/SAVE_DATA.SAVE_DATA_C"))
  (set `/Game/D-PET/CHARACTERS/SAVE_DATA.STATE` (`self.STATE`) _returnvalue)
  (set `/Game/D-PET/CHARACTERS/SAVE_DATA.PET LINE` (`self.PET LINE`) _returnvalue)
  (set `/Game/D-PET/CHARACTERS/SAVE_DATA.FIGHTS` (`self.FIGHTS`) _returnvalue)
  (set `/Game/D-PET/CHARACTERS/SAVE_DATA.AGE` (`self.AGE`) _returnvalue)
  (`GameplayStatics.SaveGameToSlot` _returnvalue "SAVE"))

(fn `UserConstructionScript`)