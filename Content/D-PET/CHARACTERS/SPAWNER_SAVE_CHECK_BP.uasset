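; Spawner actor that restores the player's pet from the "SAVE" slot on BeginPlay, or spawns an egg if the save has no pet.
; It picks a child, adult or mega class from the saved pet line and growth state, spawns it at its own transform, copies the fight count, then destroys itself.
; The SNAKE and OGRE branches currently spawn the same CROC classes.
; A missing or invalid save spawns nothing.
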(event `self.ReceiveBeginPlay`
  (bind _pet_line (`/Game/D-PET/CHARACTERS/SAVE_DATA.PET LINE` (`self.As SAVE DATA`)))
  (bind _state (`/Game/D-PET/CHARACTERS/SAVE_DATA.STATE` (`self.As SAVE DATA`)))
  (bind _state_2 (`/Game/D-PET/CHARACTERS/SAVE_DATA.STATE` (`self.As SAVE DATA`)))
  (bind _state_3 (`/Game/D-PET/CHARACTERS/SAVE_DATA.STATE` (`self.As SAVE DATA`)))
  (bind _returnvalue (`GameplayStatics.LoadGameFromSlot` "SAVE"))
  (bind _assave_data (cast `/Game/D-PET/CHARACTERS/SAVE_DATA` _returnvalue))
  (bind _output_get (set `self.As SAVE DATA` _assave_data))
  (if (`/Game/D-PET/CHARACTERS/SAVE_DATA.HAS PET ?` _output_get)
    (if (== _pet_line "CROC")
      (if (<= _state_2 1.0)
        (bind _returnvalue_2 (`|SpawnActorFromClass` "/Game/D-PET/CHARACTERS/CROC/CROC_CHILD_BP.CROC_CHILD_BP_C" (`SceneComponent.K2_GetComponentToWorld` (`self.DefaultSceneRoot`)) "Undefined" "MultiplyWithRoot" null null))
        (set `/Game/D-PET/CHARACTERS/PARENT_PET_BP.FIGHTS` (`/Game/D-PET/CHARACTERS/SAVE_DATA.FIGHTS` (`self.As SAVE DATA`)) _returnvalue_2)
        (`self.K2_DestroyActor` :!label _label)
        (elif (== _state_2 2.0)
          (bind _returnvalue_3 (`|SpawnActorFromClass` "/Game/D-PET/CHARACTERS/CROC/CROC_ADULT_BP.CROC_ADULT_BP_C" (`SceneComponent.K2_GetComponentToWorld` (`self.DefaultSceneRoot`)) "Undefined" "MultiplyWithRoot" null null))
          (set `/Game/D-PET/CHARACTERS/PARENT_PET_BP.FIGHTS` (`/Game/D-PET/CHARACTERS/SAVE_DATA.FIGHTS` (`self.As SAVE DATA`)) _returnvalue_3)
          (goto _label)
          (elif (>= _state_2 3.0)
            (bind _returnvalue_4 (`|SpawnActorFromClass` "/Game/D-PET/CHARACTERS/CROC/CROC_MEGA_BP.CROC_MEGA_BP_C" (`SceneComponent.K2_GetComponentToWorld` (`self.DefaultSceneRoot`)) "Undefined" "MultiplyWithRoot" null null))
            (set `/Game/D-PET/CHARACTERS/PARENT_PET_BP.FIGHTS` (`/Game/D-PET/CHARACTERS/SAVE_DATA.FIGHTS` (`self.As SAVE DATA`)) _returnvalue_4)
            (goto _label))))
      (elif (== _pet_line "SNAKE")
        (if (<= _state_3 1.0)
          (bind _returnvalue_5 (`|SpawnActorFromClass` "/Game/D-PET/CHARACTERS/CROC/CROC_CHILD_BP.CROC_CHILD_BP_C" (`SceneComponent.K2_GetComponentToWorld` (`self.DefaultSceneRoot`)) "Undefined" "MultiplyWithRoot" null null))
          (set `/Game/D-PET/CHARACTERS/PARENT_PET_BP.FIGHTS` (`/Game/D-PET/CHARACTERS/SAVE_DATA.FIGHTS` (`self.As SAVE DATA`)) _returnvalue_5)
          (goto _label)
          (elif (== _state_3 2.0)
            (bind _returnvalue_6 (`|SpawnActorFromClass` "/Game/D-PET/CHARACTERS/CROC/CROC_ADULT_BP.CROC_ADULT_BP_C" (`SceneComponent.K2_GetComponentToWorld` (`self.DefaultSceneRoot`)) "Undefined" "MultiplyWithRoot" null null))
            (set `/Game/D-PET/CHARACTERS/PARENT_PET_BP.FIGHTS` (`/Game/D-PET/CHARACTERS/SAVE_DATA.FIGHTS` (`self.As SAVE DATA`)) _returnvalue_6)
            (goto _label)
            (elif (>= _state_3 3.0)
              (bind _returnvalue_7 (`|SpawnActorFromClass` "/Game/D-PET/CHARACTERS/CROC/CROC_MEGA_BP.CROC_MEGA_BP_C" (`SceneComponent.K2_GetComponentToWorld` (`self.DefaultSceneRoot`)) "Undefined" "MultiplyWithRoot" null null))
              (set `/Game/D-PET/CHARACTERS/PARENT_PET_BP.FIGHTS` (`/Game/D-PET/CHARACTERS/SAVE_DATA.FIGHTS` (`self.As SAVE DATA`)) _returnvalue_7)
              (goto _label))))
        (elif (== _pet_line "OGRE")
          (if (<= _state 1.0)
            (bind _returnvalue_8 (`|SpawnActorFromClass` "/Game/D-PET/CHARACTERS/CROC/CROC_CHILD_BP.CROC_CHILD_BP_C" (`SceneComponent.K2_GetComponentToWorld` (`self.DefaultSceneRoot`)) "Undefined" "MultiplyWithRoot" null null))
            (set `/Game/D-PET/CHARACTERS/PARENT_PET_BP.FIGHTS` (`/Game/D-PET/CHARACTERS/SAVE_DATA.FIGHTS` (`self.As SAVE DATA`)) _returnvalue_8)
            (goto _label)
            (elif (== _state 2.0)
              (bind _returnvalue_9 (`|SpawnActorFromClass` "/Game/D-PET/CHARACTERS/CROC/CROC_ADULT_BP.CROC_ADULT_BP_C" (`SceneComponent.K2_GetComponentToWorld` (`self.DefaultSceneRoot`)) "Undefined" "MultiplyWithRoot" null null))
              (set `/Game/D-PET/CHARACTERS/PARENT_PET_BP.FIGHTS` (`/Game/D-PET/CHARACTERS/SAVE_DATA.FIGHTS` (`self.As SAVE DATA`)) _returnvalue_9)
              (goto _label)
              (elif (>= _state 3.0)
                (bind _returnvalue_10 (`|SpawnActorFromClass` "/Game/D-PET/CHARACTERS/CROC/CROC_MEGA_BP.CROC_MEGA_BP_C" (`SceneComponent.K2_GetComponentToWorld` (`self.DefaultSceneRoot`)) "Undefined" "MultiplyWithRoot" null null))
                (set `/Game/D-PET/CHARACTERS/PARENT_PET_BP.FIGHTS` (`/Game/D-PET/CHARACTERS/SAVE_DATA.FIGHTS` (`self.As SAVE DATA`)) _returnvalue_10)
                (goto _label)))))))
    (else
      (`|SpawnActorFromClass` "/Game/D-PET/CHARACTERS/EGG_BP.EGG_BP_C" (`SceneComponent.K2_GetComponentToWorld` (`self.DefaultSceneRoot`)) "Undefined" "OverrideRootScale" null null)
      (`self.K2_DestroyActor`))))

(fn `UserConstructionScript`)